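; BP_OfficeEnterCutscene is a one-shot overlap trigger that starts the office fall cutscene when the player character enters it.
; BeginPlay pre-creates a level sequence player for LS_OfficeFall.
; On overlap it plays the sequence and calls TheFallCutsceneStart on BP_FirstPersonCharacter.
; It then destroys itself and adds the W_Cutscene_BlackBars widget to the player screen, with the widget created after the DestroyActor call.
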(event EventBeginPlay
  (bind _returnvalue (Sequencer|Player|CreateLevelSequencePlayer "/Game/LS_OfficeFall.LS_OfficeFall"))
  (Variables|Default|SetCutscene _returnvalue))

(event Collision|EventActorBeginOverlap
  (params (OtherActor :type Actor%20Object%20Reference))
  (if (== OtherActor (Game|GetPlayerCharacter 0))
    (Sequencer|Player|Play (Variables|Default|GetCutscene) :!class /Script/MovieScene.MovieSceneSequencePlayer)
    (bind _asbp_first_person_character (Utilities|Casting|CastToBP_FirstPersonCharacter OtherActor))
    (Default|TheFallCutsceneStart _asbp_first_person_character)
    (Actor|DestroyActor)
    (bind _returnvalue (UserInterface|CreateWidget "/Game/UI/Cutscenes/W_Cutscene_BlackBars.W_Cutscene_BlackBars_C"))
    (UserInterface|Viewport|AddtoPlayerScreen _returnvalue)))

(event EventTick
  (params (DeltaSeconds :type Float%20%28single-precision%29)))

(fn ConstructionScript)