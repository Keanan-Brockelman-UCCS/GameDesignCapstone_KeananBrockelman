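; BP_LazerWall is a laser wall hazard that respawns the player on contact.
; On actor overlap it checks for player character 0, casts it to BP_FirstPersonCharacter and calls its Respawn function.
; At BeginPlay it sizes its two rect lights from the cube mesh's world X and Z scale, so the lighting matches the wall's dimensions.
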(event EventBeginPlay
  (bind _rectlight (Variables|Default|GetRectLight))
  (bind _rectlight1 (Variables|Default|GetRectLight1))
  (bind _cubemesh (Variables|Default|GetCubeMesh))
  (bind _returnvalue (Transformation|GetWorldScale _cubemesh))
  (bind _returnvalue_2 (* (.x _returnvalue) 1e+02))
  (bind _returnvalue_3 (* (.z _returnvalue) 1e+02))
  ;[0.15 0.15 0.15 0.5] Set the Rect Light Size To Match The Object's
  (Class|RectLightComponent|SetSourceWidth _rectlight _returnvalue_2)
  (Class|RectLightComponent|SetSourceHeight _rectlight _returnvalue_3)
  (Class|RectLightComponent|SetSourceWidth _rectlight1 _returnvalue_2)
  (Class|RectLightComponent|SetSourceHeight _rectlight1 _returnvalue_3))

(event Collision|EventActorBeginOverlap
  (params (OtherActor :type Actor%20Object%20Reference))
  (if (== OtherActor (Game|GetPlayerCharacter 0))
    (bind _asbp_first_person_character (Utilities|Casting|CastToBP_FirstPersonCharacter OtherActor))
    (Default|Respawn _asbp_first_person_character)))

(event EventTick
  (params (DeltaSeconds :type Float%20%28single-precision%29)))

(fn ConstructionScript)