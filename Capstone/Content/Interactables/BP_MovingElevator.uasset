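; Moving elevator that shuttles a platform between start and end marker locations when called by a podium.
; On BeginPlay it caches both locations and attaches child actors to the platform root, setting the timeline rate from travel duration inside that loop.
; An interface call plays or reverses the timeline, lerping the platform's position.
; It ignores calls while moving and messages the podium at start and finish to toggle its interact key.
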(event EventBeginPlay
  ;[0.15 0.15 0.15 0.5] Set Variables to hold the start and end locations
  (Variables|Default|SetStartingLocation (Transformation|GetWorldLocation (Variables|Default|GetStartPlatformLocation)))
  (Variables|Default|SetEndingLocation (Transformation|GetWorldLocation (Variables|Default|GetEndPlatformLocation)))
  ;[0.15 0.15 0.15 0.5] Set starting bools
  (Variables|Default|SetAtStartLocation? true)
  (Variables|Default|SetMoveInProgress false)
  ;[0.15 0.15 0.15 0.5] Keeps attached objects connected to the root if attached in the inspector
  (for _array_element (Actor|GetAttachedActors true false)
    (Transformation|AttachComponentToComponent _array_element (Variables|Default|GetPlatform_Root) "None" "KeepWorld" "KeepWorld" "KeepRelative" true)
    ;[0.15 0.15 0.15 0.5] Set
    (Components|Timeline|SetPlayRate (Variables|Default|GetMoveElevatorTimeline) (/ 1.0 (Variables|Default|GetElevator%20Travel%20Duration)))))

(event EventPodiumCommunicatewithElevator
  (params (PodiumReference :type Actor%20Object%20Reference))
  ;[0.15 0.15 0.15 0.5] Move the elevator using a timeline using the prior interfaces while also using interfaces to turn off the interact key when it is moving
  (Variables|Default|SetCallButtonReference PodiumReference)
  (if (not (Variables|Default|GetMoveInProgress))
    (Class|BPIButtonPressInteraction|ElevatorCommunicatewithPodium(Message) (Variables|Default|GetCallButtonReference) true)
    (Variables|Default|SetMoveInProgress true)
    (if (Variables|Default|GetAtStartLocation?)
      (bind (_direction _movecontribution) (Timeline|MoveElevatorTimeline PlayFromStart)
        (:Update
          (Transformation|SetWorldLocation (Variables|Default|GetPlatform_Root) (Math|Vector|Lerp(Vector) (Variables|Default|GetStartingLocation) (Variables|Default|GetEndingLocation) _movecontribution) false false))
        (:Finished
          (Variables|Default|SetMoveInProgress false)
          (Variables|Default|SetAtStartLocation? (Utilities|Select :Index _direction :Forward false :Backward true))
          (Class|BPIButtonPressInteraction|ElevatorCommunicatewithPodium(Message) (Variables|Default|GetCallButtonReference) false)))
      (else
        (Timeline|MoveElevatorTimeline ReverseFromEnd)))))

(fn ConstructionScript)