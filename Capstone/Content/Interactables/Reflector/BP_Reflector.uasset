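; BP_Reflector is a bounce pad that launches the first-person player along the Cylinder's up vector with a ReflectBoost strength.
; Overlap begin and end call the bounce functions on BP_FirstPersonCharacter, which owns the bounce and jump-reset logic.
; On BeginPlay it sizes two rect lights to the mesh scale and creates a dynamic material whose plus-pattern tiling comes from WidthT and HeightT, or from scale if either is zero.
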(event EventBeginPlay
  (bind _cylinder (Variables|Default|GetCylinder))
  (bind _cylinder_2 (Variables|Default|GetCylinder))
  (bind _cylinder_3 (Variables|Default|GetCylinder))
  (bind _rectlight1 (Variables|Default|GetRectLight1))
  (bind _rectlight (Variables|Default|GetRectLight))
  (bind _returnvalue (Transformation|GetWorldScale _cylinder))
  (bind _returnvalue_2 (Transformation|GetWorldScale _cylinder_3))
  (bind _returnvalue_3 (* (.x _returnvalue) 1e+02))
  (bind _returnvalue_4 (* (.z _returnvalue) 1e+02))
  (Utilities|FlowControl|Sequence
    (:then_0
      ;[0.15 0.15 0.15 0.5] Set the Rect Light Size To Match The Object's
      (Class|RectLightComponent|SetSourceWidth _rectlight _returnvalue_3)
      (Class|RectLightComponent|SetSourceHeight _rectlight _returnvalue_4)
      (Class|RectLightComponent|SetSourceWidth _rectlight1 _returnvalue_3)
      (Class|RectLightComponent|SetSourceHeight _rectlight1 _returnvalue_4))
    (:then_1
      ;[0.15 0.15 0.15 0.5] Creating and Setting a Dynamic Material that will create +'s based on size dynamically or by choice
      (if (or (== (Variables|Default|GetWidthT) 0.0) (== (Variables|Default|GetHeightT) 0.0))
        (bind _returnvalue_5 (Rendering|Material|CreateDynamicMaterialInstance (Rendering|Material|GetMaterial _cylinder_3 0) "None" "None" :!class /Script/Engine.KismetMaterialLibrary))
        (Rendering|Material|SetScalarParameterValue _returnvalue_5 "WidthT" (Math|Conversions|ToFloat(Integer) (Math|Float|Round (* (Math|Float|Max(Float) (.x _returnvalue_2) (.z _returnvalue_2)) 1.0))) :!class /Script/Engine.MaterialInstanceDynamic)
        (Rendering|Material|SetScalarParameterValue _returnvalue_5 "HeightT" (Math|Conversions|ToFloat(Integer) (Math|Float|Round (* (.y _returnvalue_2) 1.0))) :!class /Script/Engine.MaterialInstanceDynamic)
        (Rendering|Material|SetMaterial _cylinder_3 0 _returnvalue_5)
        (else
          (bind _returnvalue_6 (Rendering|Material|CreateDynamicMaterialInstance (Rendering|Material|GetMaterial _cylinder_2 0) "None" "None" :!class /Script/Engine.KismetMaterialLibrary))
          (Rendering|Material|SetScalarParameterValue _returnvalue_6 "WidthT" (Variables|Default|GetWidthT) :!class /Script/Engine.MaterialInstanceDynamic)
          (Rendering|Material|SetScalarParameterValue _returnvalue_6 "HeightT" (Variables|Default|GetHeightT) :!class /Script/Engine.MaterialInstanceDynamic)
          (Rendering|Material|SetMaterial _cylinder_2 0 _returnvalue_6))))))

(event Collision|EventActorBeginOverlap
  (params (OtherActor :type Actor%20Object%20Reference))
  ;[0.15 0.15 0.15 0.5] Bounces Player in Player Script
  (if (== OtherActor (Game|GetPlayerCharacter 0))
    (bind _asbp_first_person_character (Utilities|Casting|CastToBP_FirstPersonCharacter OtherActor))
    (Default|StartBounceCollision _asbp_first_person_character (Math|Vector|GetUpVector (Variables|Default|GetCylinder)) (Variables|Default|GetReflect%20Boost))))

(event EventTick
  (params (DeltaSeconds :type Float%20%28single-precision%29)))

(event Collision|EventActorEndOverlap
  (params (OtherActor :type Actor%20Object%20Reference))
  ;[0.15 0.15 0.15 0.5] Resets Player Jump in the Player Script
  (if (== OtherActor (Game|GetPlayerCharacter 0))
    (bind _asbp_first_person_character (Utilities|Casting|CastToBP_FirstPersonCharacter OtherActor))
    (Default|EndBounceCollision _asbp_first_person_character)))

(fn ConstructionScript)