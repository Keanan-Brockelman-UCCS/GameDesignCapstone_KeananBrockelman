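; Elevator call button podium that shows a billboard prompt while a Character overlaps its sphere.
; On interaction from the character, it messages the referenced elevator if allowed and calls CloseDoor on all ElevatorDoorLeft actors in the level.
; The elevator reports progress back, which blocks interaction and hides the prompt while moving, then re-enables both.
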(event OnComponentBeginOverlap(Sphere)
  (params (OverlappedComponent :type Primitive%20Component%20Object%20Reference) (OtherActor :type Actor%20Object%20Reference) (OtherComp :type Primitive%20Component%20Object%20Reference) (OtherBodyIndex :type Integer) (bFromSweep :type Boolean) (SweepResult :type Hit%20Result%20Structure%20%28by%20ref%29))
  ;[0.15 0.15 0.15 0.5] Turn On/Off Button Prompt
  (CallFunction|TestforCharacterandSetVisibility OtherActor true))

(event OnComponentEndOverlap(Sphere)
  (params (OverlappedComponent :type Primitive%20Component%20Object%20Reference) (OtherActor :type Actor%20Object%20Reference) (OtherComp :type Primitive%20Component%20Object%20Reference) (OtherBodyIndex :type Integer))
  ;[0.15 0.15 0.15 0.5] Turn On/Off Button Prompt
  (CallFunction|TestforCharacterandSetVisibility OtherActor false))

(event EventBeginPlay
  (Rendering|SetVisibility (Variables|Default|GetBillboard) false false) ; Set the visibility of the Button Prompt to False On Start
)

(event EventElevatorCommunicatewithPodium
  (params (IsInProgress? :type Boolean))
  (bind _returnvalue (not IsInProgress?))
  ;[0.15 0.15 0.15 0.5] Set Visibility of interaction prompt off when the elevator is going
  (Variables|Default|SetAllow%20Interaction? _returnvalue)
  (Rendering|SetVisibility (Variables|Default|GetBillboard) _returnvalue false))

(event EventCharacterInteractwithWorldObject
  ;[0.15 0.15 0.15 0.5] Called from Character then communicate to Elevator
  (if (Variables|Default|GetAllow%20Interaction?)
    (bind _elevatorreference (Variables|Default|GetElevatorReference)
      (:then
        (Class|BPIButtonPressInteraction|PodiumCommunicatewithElevator(Message) _elevatorreference self)
        ;[0.15 0.15 0.15 0.5] Close Elevator Door
        (bind _outactors (Actor|GetAllActorsOfClass "/Game/ElevatorDoorLeft.ElevatorDoorLeft_C"))
        (Default|CloseDoor _outactors))
      (:else))))

(fn ConstructionScript)

(fn TestforCharacterandSetVisibility
  (params (Object :type Object%20Object%20Reference) (bNewVisibility :type Boolean))
  (Utilities|Casting|CastToCharacter Object)
  (Rendering|SetVisibility (Variables|Default|GetBillboard) bNewVisibility false))