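; BP_LeadingLightCorrect is a leading-light actor that fades away and destroys itself when the player character overlaps it.
; At BeginPlay it puts a dynamic material instance on the light ray cone mesh.
; A timeline drives the fade, setting the cone's opacity and multiplying the spotlight's current intensity by the track value on every update, so the dimming compounds.
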(event Custom|FadeAway
  (bind _spotlight (Variables|Default|GetSpotLight))
  (bind _time (Timeline|LightFadeTimeline PlayFromStart)
    (:Update
      (Rendering|Components|Light|SetIntensity _spotlight (* (Variables|/Script/Engine.LightComponentBase|GetIntensity _spotlight) _time))
      (Rendering|Material|SetScalarParameterValue (Variables|Default|GetDynamicMaterial) "Opacity" _time :!class /Script/Engine.MaterialInstanceDynamic))
    (:Finished
      (Actor|DestroyActor))))

(event EventBeginPlay
  (bind _lightraycone (Variables|Default|GetLightRayCone))
  (bind _returnvalue (Rendering|Material|CreateDynamicMaterialInstance (Rendering|Material|GetMaterial _lightraycone 0) "None" "None" :!class /Script/Engine.KismetMaterialLibrary))
  (bind _output_get (Variables|Default|SetDynamicMaterial _returnvalue))
  (Rendering|Material|SetMaterial _lightraycone 0 _output_get))

(event Collision|EventActorBeginOverlap
  (params (OtherActor :type Actor%20Object%20Reference))
  (if (== OtherActor (Game|GetPlayerCharacter 0))
    (CallFunction|FadeAway)))

(event EventTick
  (params (DeltaSeconds :type Float%20%28single-precision%29)))

(fn ConstructionScript)