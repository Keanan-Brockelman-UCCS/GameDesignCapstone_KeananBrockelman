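; BP_LazerWall is a laser wall hazard that respawns the player's first-person character when it begins overlapping the wall.
; On BeginPlay, it sizes two rect lights to the cube mesh's world scale.
; It also gives the mesh a dynamic material whose X pattern counts use WidthX and HeightX, or are derived from rounded mesh scale if either is zero.
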(event EventBeginPlay
  (bind _cubemesh (Variables|Default|GetCubeMesh))
  (bind _rectlight (Variables|Default|GetRectLight))
  (bind _cubemesh_2 (Variables|Default|GetCubeMesh))
  (bind _cubemesh_3 (Variables|Default|GetCubeMesh))
  (bind _rectlight1 (Variables|Default|GetRectLight1))
  (bind _returnvalue (Transformation|GetWorldScale _cubemesh_2))
  (bind _returnvalue_2 (Transformation|GetWorldScale _cubemesh_3))
  (bind _returnvalue_3 (* (.x _returnvalue) 1e+02))
  (bind _returnvalue_4 (* (.z _returnvalue) 1e+02))
  (Utilities|FlowControl|Sequence
    (:then_0
      ;[0.15 0.15 0.15 0.5] Set the Rect Light Size To Match The Object's
      (Class|RectLightComponent|SetSourceWidth _rectlight _returnvalue_3)
      (Class|RectLightComponent|SetSourceHeight _rectlight _returnvalue_4)
      (Class|RectLightComponent|SetSourceWidth _rectlight1 _returnvalue_3)
      (Class|RectLightComponent|SetSourceHeight _rectlight1 _returnvalue_4))
    (:then_1
      ;[0.15 0.15 0.15 0.5] Creating and Setting a Dynamic Material that will create X's based on size dynamically or by choice
      (if (or (== (Variables|Default|GetWidthX) 0.0) (== (Variables|Default|GetHeightX) 0.0))
        (bind _returnvalue_5 (Rendering|Material|CreateDynamicMaterialInstance (Rendering|Material|GetMaterial _cubemesh_3 0) "None" "None" :!class /Script/Engine.KismetMaterialLibrary))
        (Rendering|Material|SetScalarParameterValue _returnvalue_5 "WidthX" (Math|Conversions|ToFloat(Integer) (Math|Float|Round (* (Math|Float|Max(Float) (.x _returnvalue_2) (.y _returnvalue_2)) 1.0))) :!class /Script/Engine.MaterialInstanceDynamic)
        (Rendering|Material|SetScalarParameterValue _returnvalue_5 "HeightX" (Math|Conversions|ToFloat(Integer) (Math|Float|Round (* (.z _returnvalue_2) 1.0))) :!class /Script/Engine.MaterialInstanceDynamic)
        (Rendering|Material|SetMaterial _cubemesh_3 0 _returnvalue_5)
        (else
          (bind _returnvalue_6 (Rendering|Material|CreateDynamicMaterialInstance (Rendering|Material|GetMaterial _cubemesh 0) "None" "None" :!class /Script/Engine.KismetMaterialLibrary))
          (Rendering|Material|SetScalarParameterValue _returnvalue_6 "WidthX" (Variables|Default|GetWidthX) :!class /Script/Engine.MaterialInstanceDynamic)
          (Rendering|Material|SetScalarParameterValue _returnvalue_6 "HeightX" (Variables|Default|GetHeightX) :!class /Script/Engine.MaterialInstanceDynamic)
          (Rendering|Material|SetMaterial _cubemesh 0 _returnvalue_6))))))

(event Collision|EventActorBeginOverlap
  (params (OtherActor :type Actor%20Object%20Reference))
  (if (== OtherActor (Game|GetPlayerCharacter 0))
    (bind _asbp_first_person_character (Utilities|Casting|CastToBP_FirstPersonCharacter OtherActor))
    (Default|Respawn _asbp_first_person_character)))

(event EventTick
  (params (DeltaSeconds :type Float%20%28single-precision%29)))

(fn ConstructionScript)