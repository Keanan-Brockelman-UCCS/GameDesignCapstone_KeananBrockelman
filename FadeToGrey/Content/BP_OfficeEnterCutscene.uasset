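; BP_OfficeEnterCutscene is a one-shot trigger actor that starts the LS_OfficeFall cutscene when the player overlaps it.
; It creates the level sequence player on BeginPlay.
; On overlap it calls CutsceneRespawn and DisablePlayerMovement on BP_FirstPersonCharacter, plays the sequence and shows the W_Cutscene_BlackBars widget.
; It then destroys itself, leaving movement restoration and widget removal outside this Blueprint.
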(event EventBeginPlay
  (bind _returnvalue (Sequencer|Player|CreateLevelSequencePlayer "/Game/Levels/TheOffice/LS_OfficeFall.LS_OfficeFall"))
  (Variables|Default|SetCutscene _returnvalue))

(event Collision|EventActorBeginOverlap
  (params (OtherActor :type Actor%20Object%20Reference))
  (bind _returnvalue (Game|GetPlayerCharacter 0))
  (if (== OtherActor _returnvalue)
    (bind _asbp_first_person_character (Utilities|Casting|CastToBP_FirstPersonCharacter _returnvalue))
    (Default|CutsceneRespawn _asbp_first_person_character)
    (Default|DisablePlayerMovement _asbp_first_person_character)
    (Sequencer|Player|Play (Variables|Default|GetCutscene) :!class /Script/MovieScene.MovieSceneSequencePlayer)
    (bind _returnvalue_2 (UserInterface|CreateWidget "/Game/UI/Cutscenes/W_Cutscene_BlackBars.W_Cutscene_BlackBars_C"))
    (UserInterface|Viewport|AddtoPlayerScreen _returnvalue_2)
    (Actor|DestroyActor)))

(event EventTick
  (params (DeltaSeconds :type Float%20%28single-precision%29)))

(fn ConstructionScript)